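; BP_EnemyTower is an enemy tower that shows a temporary health bar when it takes damage.
; On BeginPlay it caches the WBP_HealthBar from its widget component and hides it.
; DamageTakenFollowUp updates the bar's percentage, makes it visible without hit testing, and sets a one-shot timer that hides it again after HealthBarTime.
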(event `self.ReceiveBeginPlay`
  (bind _aswbp_health_bar (cast `/Game/_Blueprint/Widgets/WBP_HealthBar` (`WidgetComponent.GetUserWidgetObject` (`self.Widget`))))
  (bind _output_get (set `self.HealthBarRef` _aswbp_health_bar))
  (`Widget.SetVisibility` _output_get "Hidden"))

(event `self.DamageTakenFollowUp`
  (params (HealthPercentage :type "Float (single-precision)"))
  (bind _healthbarref (`self.HealthBarRef`))
  (`KismetSystemLibrary.K2_SetTimerDelegate` (delegate `HideHealthBar`) (`self.HealthBarTime`))
  (`Widget.SetVisibility` _healthbarref "HitTestInvisible")
  (`ProgressBar.SetPercent` (`/Game/_Blueprint/Widgets/WBP_HealthBar.HealthBar` _healthbarref) HealthPercentage))

(event `HideHealthBar`
  (`Widget.SetVisibility` (`self.HealthBarRef`) "Hidden"))

(fn `UserConstructionScript`)